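; A Heart graph layout helper that automatically arranges nodes in a grid of columns.
; It drops annotation nodes, sorts the rest into trees along output links with duplicates allowed, then splits each tree into layers.
; Layers step toward negative X, nodes stack along Y within each layer, and each tree gets a fixed Y offset by index, regardless of its size.
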(fn LayoutBP
  (params (Accessor :type Heart%20Node%20Location%20Accessor%20Interface%20%28by%20ref%29) (Nodes :type Array%20of%20Heart%20Graph%20Node%20Object%20References))
  (bind _returnvalue (Class|HeartNodeSortingLibrary|FilterNodesbyClassExclusive Nodes (Utilities|Set|MakeSet "/Script/Heart.HeartGraphNodeAnnotation")))
  (bind _trees (Class|HeartNodeSortingLibrary|SortLooseNodesIntoTrees _returnvalue (Utilities|Struct|MakeNodeLooseToTreeArgs true "Output")))
  (for (_array_element _array_index) _trees
    (bind _layers (Class|HeartNodeSortingLibrary|ConvertNodeTreetoLayers _array_element))
    (for (_array_element_2 _array_index_2) _layers
      (bind _result (Utilities|Set|ToArray (Utilities|Struct|BreakHeartNodeLayer _array_element_2)))
      (for (_array_element_3 _array_index_3) _result
        (Class|HeartNodeLocationAccessor|SetNodeLocation Accessor _array_element_3 (Math|Vector2D|MakeVector2D (* _array_index_2 (Variables|Default|GetLayerSpacing) -1.0) (+ (* _array_index_3 (Variables|Default|GetNodeSpacing)) (* _array_index (Variables|Default|GetTreeSpacing))))))))
  (Development|PrintString self "LayoutHelper End")
  (return true))