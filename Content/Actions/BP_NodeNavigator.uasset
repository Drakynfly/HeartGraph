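; BP_NodeNavigator is a Heart graph action that moves selection between connected nodes with directional keys.
; It runs only on widgets implementing HeartGraphNodeInterface and converts the key event into a UI navigation direction vector.
; RunNodeNavigation picks the connected node whose location best matches that direction.
; It then replaces the canvas selection with that node, gives its displayed widget keyboard focus and reports the input as handled.
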(fn BPExecuteonNode
  (params (CanvasNode :type Heart%20Graph%20Canvas%20Node%20Object%20Reference) (Activation :type Heart%20Input%20Activation%20Structure%20%28by%20ref%29) (ContextObject :type Object%20Object%20Reference))
  (Class|HeartInputActivationLibrary|SwitchonActivationType Activation
    (:KeyEvent
      (bind _value (CallFunction|RunNodeNavigation (Variables|/Script/HeartCanvas.HeartGraphCanvasNode|GetGraphCanvas CanvasNode) (Variables|/Script/HeartCanvas.HeartGraphCanvasNode|GetGraphNode CanvasNode) (Class|HeartWidgetUtilsLibrary|UINavigationtoVector (Class|KismetInputLibrary|KeyGetNavigationDirectionfromKey (Class|HeartInputActivationLibrary|ActivationtoKeyEvent Activation)))))
      (return _value))))

(fn BPCanExecuteonWidget
  (params (Widget :type Heart%20Graph%20Widget%20Base%20Object%20Reference))
  (return (Utilities|DoesObjectImplementInterface Widget "/Script/Heart.HeartGraphNodeInterface")))

(fn RunNodeNavigation
  (params (Canvas :type Heart%20Graph%20Canvas%20Object%20Reference) (Node :type Heart%20Graph%20Node%20Object%20Reference) (Direction :type Vector%202D%20Structure))
  (LocalVariables|SetFromLocation (Class|HeartGraphNode|GetLocation Node))
  (bind _result (Utilities|Set|ToArray (Class|HeartGraphNode|GetConnectedGraphNodes Node)))
  (for _array_element _result
    (Utilities|Array|Add (LocalVariables|GetConnectionLocations) (Class|HeartGraphNode|GetLocation _array_element)))
  (bind _output_get (LocalVariables|SetSelectedIndex (Class|HeartWidgetUtilsLibrary|FindClosesttoDirection (LocalVariables|GetConnectionLocations) (LocalVariables|GetFromLocation) Direction 0.5)))
  (if (Utilities|Array|IsValidIndex _result _output_get)
    (Class|HeartGraphCanvas|ClearNodeSelection Canvas)
    (Class|HeartGraphCanvas|SelectNode Canvas (Class|HeartGraphNode|GetGuid (Utilities|Array|Get(acopy) _result _output_get)))
    (Widget|SetKeyboardFocus (.Value (Utilities|Map|Find (Variables|/Script/HeartCanvas.HeartGraphCanvas|GetDisplayedNodes Canvas) (Class|HeartGraphNode|GetGuid (Utilities|Array|Get(acopy) _result _output_get)))))
    (return (Class|WidgetBlueprintLibrary|Handled))))