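; Editor-style action for Heart graph canvases that deletes the node it is executed on, described as "Delete Node".
; It is available only on Heart graph canvas node widgets whose graph node reports that it can be deleted.
; Execution removes the node from the canvas's graph by its GUID and reports the action as handled.
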(fn BPExecuteonNode
  (params (CanvasNode :type Heart%20Graph%20Canvas%20Node%20Object%20Reference) (Activation :type Heart%20Input%20Activation%20Structure%20%28by%20ref%29) (ContextObject :type Object%20Object%20Reference))
  (Class|HeartGraph|RemoveNode (Class|HeartGraphCanvas|GetGraph (Variables|/Script/HeartCanvas.HeartGraphCanvasNode|GetGraphCanvas CanvasNode)) (Class|HeartGraphNode|GetGuid (Variables|/Script/HeartCanvas.HeartGraphCanvasNode|GetGraphNode CanvasNode)))
  (return (Class|WidgetBlueprintLibrary|Handled)))

(fn BPCanExecuteonWidget
  (params (Widget :type Heart%20Graph%20Widget%20Base%20Object%20Reference))
  (bind _asheart_graph_canvas_node (Utilities|Casting|CastToHeartGraphCanvasNode Widget)
    (:then
      (return (Class|HeartGraphNode|CanDelete (Variables|/Script/HeartCanvas.HeartGraphCanvasNode|GetGraphNode _asheart_graph_canvas_node))))
    (:CastFailed
      (return false))))

(fn BPGetDescription
  (params (Widget :type Heart%20Graph%20Widget%20Base%20Object%20Reference))
  (return "Delete Node"))